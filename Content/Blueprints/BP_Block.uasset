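; BP_Block is a breakable block that loses a life each time a BP_Ball hits it.
; At one life left the Cube mesh switches to a different material to show damage.
; At zero lives it has a weighted random chance to spawn a BP_Bonus at its location, then destroys itself.
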(event EventBeginPlay)

(event Collision|EventActorBeginOverlap
  (params (OtherActor :type Actor%20Object%20Reference)))

(event EventTick
  (params (DeltaSeconds :type Float%20%28single-precision%29)))

(event Collision|EventHit
  (params (MyComp :type Primitive%20Component%20Object%20Reference) (Other :type Actor%20Object%20Reference) (OtherComp :type Primitive%20Component%20Object%20Reference) (bSelfMoved :type Boolean) (HitLocation :type Vector :default "0, 0, 0") (HitNormal :type Vector :default "0, 0, 0") (NormalImpulse :type Vector :default "0, 0, 0") (Hit :type Hit%20Result%20Structure%20%28by%20ref%29))
  (Utilities|Casting|CastToBP_Ball Other)
  (bind _output_get (Variables|Default|SetLives (- (Variables|Default|GetLives) 1)))
  (if (== _output_get 1)
    (Rendering|Material|SetMaterial (Variables|Default|GetCube) 0 "/Engine/VREditor/BasicMeshes/MI_Cube_03.MI_Cube_03")
    (elif (== (Variables|Default|GetLives) 0)
      (CallFunction|SpawnBonus)
      (Actor|DestroyActor))))

(fn ConstructionScript)

(fn SpawnBonus
  (if (Math|Random|RandomBoolwithWeight 0.3)
    (Game|SpawnActorfromClass "/Game/Blueprints/BP_Bonus.BP_Bonus_C" (Math|Transform|MakeTransform (Transformation|GetActorLocation) "0, 0, 0" "1.000000,1.000000,1.000000") "Undefined" "MultiplyWithRoot" 0 0)))