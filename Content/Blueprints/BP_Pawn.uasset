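; Player paddle pawn for a ball game that moves sideways and spawns the balls.
; MoveRight input applies a swept world offset by the Speed vector, flipping its Y for positive input, with no delta-time scaling.
; BeginPlay spawns a BP_Ball at the capsule and binds an event to its OnDead dispatcher.
; Overlapping a BP_Bonus spawns a BP_BonusBall at the capsule and destroys the pickup.
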(event EventBeginPlay
  (CallFunction|SpawnBall))

(event Collision|EventActorBeginOverlap
  (params (OtherActor :type Actor%20Object%20Reference))
  (bind _asbp_bonus (Utilities|Casting|CastToBP_Bonus OtherActor))
  (CallFunction|SpawnBonusBall)
  (Actor|DestroyActor _asbp_bonus))

(event EventTick
  (params (DeltaSeconds :type Float%20%28single-precision%29)))

(event Input|AxisEvents|InputAxisMoveRight
  (params (AxisValue :type Float%20%28single-precision%29))
  (if (> AxisValue 0.0)
    (Transformation|AddActorWorldOffset (* (Variables|Default|GetSpeed) "1.000000,-1.000000,1.000000") true)))

(event Input|AxisEvents|InputAxisMoveRight
  (params (AxisValue :type Float%20%28single-precision%29))
  (if (< AxisValue 0.0)
    (Transformation|AddActorWorldOffset (Variables|Default|GetSpeed) true)))

(fn ConstructionScript)

(fn SpawnBall
  (bind _returnvalue (Game|SpawnActorfromClass "/Game/Blueprints/BP_Ball.BP_Ball_C" (Math|Transform|MakeTransform (Transformation|GetWorldLocation (Variables|Default|GetCapsule)) "0, 0, 0" "1.000000,1.000000,1.000000") "Undefined" "MultiplyWithRoot" 0 0))
  (bind _output_get (Variables|Default|SetNewBall _returnvalue))
  (EventDispatchers|BindEventtoOnDead _output_get (EventDispatchers|CreateEvent :!event SpawnBall)))

(fn SpawnBonusBall
  (Game|SpawnActorfromClass "/Game/Blueprints/BP_BonusBall.BP_BonusBall_C" (Math|Transform|MakeTransform (Transformation|GetWorldLocation (Variables|Default|GetCapsule)) "0, 0, 0" "1.000000,1.000000,1.000000") "Undefined" "MultiplyWithRoot" 0 0))